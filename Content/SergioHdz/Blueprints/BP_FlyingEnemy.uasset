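; BP_FlyingEnemy is a flying enemy that drifts between preset points while firing bullets.
; Every 1.5–2.5 seconds it picks one of three arrow positions and a new random yaw spin, applied on Tick.
; A repeating Moving timer eases the skeletal mesh toward that point by a fixed lerp fraction.
; Every two seconds it spawns BP_BulletFlyEn from Arrow6, rotated using its and the player's forward vectors, not positions.
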(event Custom|Moving
  (bind _skeletalmesh (Variables|Default|GetSkeletalMesh))
  (Variables|Default|SetAlpha 0.0)
  (Utilities|Time|SetTimerbyEvent (delegate Custom|Moving) 0.02)
  (Variables|Default|SetAlpha (+ (Variables|Default|GetAlpha) 0.02))
  (Transformation|SetWorldLocation _skeletalmesh (Math|Vector|Lerp(Vector) (Transformation|GetWorldLocation _skeletalmesh) (Variables|Default|GetLocationToMove) (Variables|Default|GetAlpha)) false false))

(event Custom|FindNextLocation
  (bind _arrow1 (Variables|Default|GetArrow1))
  (bind _arrow2 (Variables|Default|GetArrow2))
  (bind _arrow3 (Variables|Default|GetArrow3))
  (bind _array (Utilities|Array|MakeArray _arrow1 _arrow2 _arrow3))
  (Variables|Default|SetDelta%20Rotation%20Z%20%28Yaw%29 (Math|Random|RandomFloatinRange -5.0 5.0))
  (Variables|Default|SetLocationToMove (Transformation|GetWorldLocation (Utilities|Array|Get(acopy) _array (Math|Random|RandomIntegerinRange 0 (Utilities|Array|LastIndex _array)))))
  (CallFunction|Moving)
  (Utilities|FlowControl|Delay (Math|Random|RandomFloatinRange 1.5 2.5))
  (CallFunction|FindNextLocation))

(event Custom|Shooting
  (bind _arrow6 (Variables|Default|GetArrow6))
  (Transformation|SetWorldRotation _arrow6 (Math|Rotator|FindLookatRotation (Math|Rotator|GetRotationXVector (Transformation|GetWorldRotation _arrow6)) (Math|Rotator|GetRotationXVector (Transformation|GetWorldRotation (Variables|/Script/Engine.Actor|GetRootComponent (Game|Player|GetPlayerPawn 0))))) false false)
  (Game|SpawnActorfromClass "/Game/SergioHdz/Blueprints/BP_BulletFlyEn.BP_BulletFlyEn_C" (Transformation|GetWorldTransform (Variables|Default|GetArrow6)) "Undefined" "MultiplyWithRoot" 0 0))

(event EventBeginPlay
  (CallFunction|FindNextLocation)
  (CallFunction|Shooting :!label _label)
  (Utilities|FlowControl|Delay 2.0)
  (goto _label))

(event Collision|EventActorBeginOverlap
  (params (OtherActor :type Actor%20Object%20Reference)))

(event EventTick
  (params (DeltaSeconds :type Float%20%28single-precision%29))
  (Transformation|AddLocalRotation (Variables|Default|GetSkeletalMesh) (Math|Rotator|MakeRotator 0.0 0.0 (Variables|Default|GetDelta%20Rotation%20Z%20%28Yaw%29)) false false))

(fn ConstructionScript)