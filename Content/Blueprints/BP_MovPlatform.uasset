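; BP_MovPlatform is an actor that oscillates back and forth along one horizontal world axis as a moving platform.
; BeginPlay records the start location, and Tick offsets from it with a sine on X or, when SwitchAxis is set, a cosine on Y.
; Game time scaled by MoveSpeed drives the wave, XDistance or YDistance sets the amplitude, and each move sweeps for collision.
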(event EventBeginPlay
  (Variables|Default|SetStartLocation (Transformation|GetActorLocation self)))

(event Collision|EventActorBeginOverlap
  (params (OtherActor :type Actor%20Object%20Reference)))

(event EventTick
  (params (DeltaSeconds :type Float%20%28single-precision%29))
  (if (Variables|Default|GetbSwitchAxis)
    (Transformation|SetActorLocation (+ (Variables|Default|GetStartLocation) (Math|Vector|MakeVector 0.0 (* (Math|Trig|Cos(Radians) (* (Utilities|Time|GetGameTimeinSeconds) (Variables|Default|GetMoveSpeed))) (Variables|Default|GetYDistance)) 0.0)) true false)
    (else
      (Transformation|SetActorLocation (+ (Variables|Default|GetStartLocation) (Math|Vector|MakeVector (* (Math|Trig|Sin(Radians) (* (Utilities|Time|GetGameTimeinSeconds) (Variables|Default|GetMoveSpeed))) (Variables|Default|GetXDistance)) 0.0 0.0)) true false))))

(fn ConstructionScript)