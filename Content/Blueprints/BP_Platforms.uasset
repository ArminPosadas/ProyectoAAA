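; BP_Platforms is a breakable platform actor that disappears when touched and respawns after a delay.
; Its Box overlap triggers BreakPlatform for actors tagged Enemy, or also Player when BreakOnPlayer is enabled.
; Breaking hides the whole component hierarchy and disables collision, then restores both after RespawnTime, with an IsBroken flag blocking retriggers meanwhile.
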(event OnComponentBeginOverlap(Box)
  (params (OverlappedComponent :type Primitive%20Component%20Object%20Reference) (OtherActor :type Actor%20Object%20Reference) (OtherComp :type Primitive%20Component%20Object%20Reference) (OtherBodyIndex :type Integer) (bFromSweep :type Boolean) (SweepResult :type Hit%20Result%20Structure%20%28by%20ref%29))
  (bind _returnvalue (Actor|ActorHasTag OtherActor "Enemy"))
  (if (not (Variables|Default|GetbIsBroken))
    (if (Variables|Default|GetbBreakOnPlayer)
      (if (or (Actor|ActorHasTag OtherActor "Player") _returnvalue)
        (CallFunction|BreakPlatform :!label _label))
      (elif _returnvalue
        (goto _label)))))

(event Custom|BreakPlatform
  (bind _defaultsceneroot (Variables|Default|GetDefaultSceneRoot))
  (Variables|Default|SetbIsBroken true)
  (Rendering|SetVisibility _defaultsceneroot false true)
  (Collision|SetActorEnableCollision false)
  (Utilities|FlowControl|Delay (Variables|Default|GetRespawnTime))
  (Rendering|SetVisibility _defaultsceneroot true true)
  (Collision|SetActorEnableCollision true)
  (Variables|Default|SetbIsBroken false))

(event EventBeginPlay
  (Variables|Default|SetbIsBroken false)
  (Rendering|SetVisibility (Variables|Default|GetDefaultSceneRoot) true true)
  (Collision|SetActorEnableCollision true))

(event Collision|EventActorBeginOverlap
  (params (OtherActor :type Actor%20Object%20Reference)))

(event EventTick
  (params (DeltaSeconds :type Float%20%28single-precision%29)))

(fn ConstructionScript)