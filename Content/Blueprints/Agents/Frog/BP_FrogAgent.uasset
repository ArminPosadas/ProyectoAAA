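; BP_FrogAgent is an AI-controlled frog enemy that damages the player on contact.
; It caches its AI_Frog controller at BeginPlay and clears that controller's IsAlive each tick while its own is false.
; Sphere overlap sends Damage to player-tagged actors, Attack sets CanAttack with a debug print, and overlap end clears it.
; AIReceiveDamage sets HealthPoints to damage minus health while above zero, without updating IsAlive.
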(event OnComponentBeginOverlap(Sphere)
  (params (OverlappedComponent :type Primitive%20Component%20Object%20Reference) (OtherActor :type Actor%20Object%20Reference) (OtherComp :type Primitive%20Component%20Object%20Reference) (OtherBodyIndex :type Integer) (bFromSweep :type Boolean) (SweepResult :type Hit%20Result%20Structure%20%28by%20ref%29))
  (if (Actor|ActorHasTag OtherActor (Variables|Default|GetPlayerTag))
    (Class|BPIPlayerDamage|ReceiveDamage(Message) OtherActor (Variables|Default|GetDamage))))

(event OnComponentEndOverlap(Sphere)
  (params (OverlappedComponent :type Primitive%20Component%20Object%20Reference) (OtherActor :type Actor%20Object%20Reference) (OtherComp :type Primitive%20Component%20Object%20Reference) (OtherBodyIndex :type Integer))
  (if (Actor|ActorHasTag OtherActor (Variables|Default|GetPlayerTag))
    (Variables|Default|SetCanAttack false)))

(event Custom|Attack
  (Variables|Default|SetCanAttack true)
  (Development|PrintString "Ataque"))

(event EventTick
  (params (DeltaSeconds :type Float%20%28single-precision%29))
  (if (== (Variables|Default|GetIsAlive) false)
    (Variables|/Game/Blueprints/Agents/Frog/AI_Frog.AI_Frog_C|SetIsAlive (Variables|Default|GetSelfController) false)))

(event EventAIReceiveDamage
  (params (Damage :type Integer))
  (CallFunction|ReceiveDamage Damage))

(event EventBeginPlay
  (bind _asai_frog (Utilities|Casting|CastToAI_Frog (Pawn|GetController self)))
  (Variables|Default|SetSelfController _asai_frog))

(fn ConstructionScript)

(fn ReceiveDamage
  (params (Damage :type Integer))
  (if (not (<= (Variables|Default|GetHealthPoints) 0.0))
    (Variables|Default|SetHealthPoints (- Damage (Variables|Default|GetHealthPoints)))
    (return)))