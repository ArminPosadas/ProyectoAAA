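; Piranha enemy agent that damages the player on contact and is driven by an AI_Piranha controller.
; On BeginPlay it caches that controller and writes its TargetPoint into the controller's Blackboard.
; A sphere overlap with a player-tagged actor sends a damage message, without checking CanAttack.
; The Attack event sets CanAttack and prints a debug string, the player leaving the sphere clears it, and SelfDestroy destroys the actor.
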(event OnComponentBeginOverlap(Sphere)
  (params (OverlappedComponent :type Primitive%20Component%20Object%20Reference) (OtherActor :type Actor%20Object%20Reference) (OtherComp :type Primitive%20Component%20Object%20Reference) (OtherBodyIndex :type Integer) (bFromSweep :type Boolean) (SweepResult :type Hit%20Result%20Structure%20%28by%20ref%29))
  (if (Actor|ActorHasTag OtherActor (Variables|Default|GetPlayerTag))
    (Class|BPIPlayerDamage|ReceiveDamage(Message) OtherActor (Variables|Default|GetDamage))))

(event OnComponentEndOverlap(Sphere)
  (params (OverlappedComponent :type Primitive%20Component%20Object%20Reference) (OtherActor :type Actor%20Object%20Reference) (OtherComp :type Primitive%20Component%20Object%20Reference) (OtherBodyIndex :type Integer))
  (if (Actor|ActorHasTag OtherActor (Variables|Default|GetPlayerTag))
    (Variables|Default|SetCanAttack false)))

(event Custom|SelfDestroy
  (Actor|DestroyActor))

(event Custom|Attack
  (Variables|Default|SetCanAttack true)
  (Development|PrintString "Ataque"))

(event EventTick
  (params (DeltaSeconds :type Float%20%28single-precision%29)))

(event EventBeginPlay
  (bind _asai_piranha (Utilities|Casting|CastToAI_Piranha (Pawn|GetController self)))
  (bind _output_get (Variables|Default|SetSelfController _asai_piranha))
  (AI|Components|Blackboard|SetValueasObject (Variables|/Script/AIModule.AIController|GetBlackboard _output_get) (Utilities|Name|MakeLiteralName "TargetPoint") (Variables|Default|GetTargetPoint)))

(fn ConstructionScript)