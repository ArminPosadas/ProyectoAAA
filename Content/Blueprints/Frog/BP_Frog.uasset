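; Frog actor that hops to a target point using scripted movement in Tick rather than physics.
; Jumpto stores the target; once JumpStarted is also set, the frog rises in fixed per-frame steps past JumpDistance.
; It then snaps horizontally to the target and descends to its BeginPlay height, setting HasLanded.
; ResetAnimVars clears the InAir, HasLanded and JumpStarted flags, named as animation variables.
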(event EventBeginPlay
  (Variables|Default|SetOriginalZ (.z (Transformation|GetActorLocation self))))

(event EventJumpto
  (params (Position :type Vector :default "0, 0, 0"))
  (Variables|Default|SetCanJump true)
  (Variables|Default|SetJumpPoint Position))

(event EventTick
  (params (DeltaSeconds :type Float%20%28single-precision%29))
  (bind _self self)
  (bind _self_2 self)
  (bind _returnvalue (Transformation|GetActorLocation _self_2))
  (bind _returnvalue_2 (Transformation|GetActorLocation _self))
  (if (and (Variables|Default|GetCanJump) (Variables|Animation|GetJumpStarted))
    (if (<= (.z _returnvalue) (+ (Variables|Default|GetOriginalZ) (Variables|Default|GetJumpDistance)))
      (CallFunction|Jump (.x _returnvalue) (.y _returnvalue) (.z _returnvalue))
      (else
        (CallFunction|MovetoPoind)))
    (elif (Variables|Default|GetIsFalling)
      (if (<= (Variables|Default|GetOriginalZ) (.z _returnvalue_2))
        (CallFunction|Land (.x _returnvalue_2) (.y _returnvalue_2) (.z _returnvalue_2))
        (else
          (Utilities|FlowControl|Sequence
            (:then_0
              (Variables|Default|SetIsFalling false))
            (:then_1
              (Variables|Animation|SetHasLanded true))))))))

(fn ConstructionScript)

(fn Jump
  (params (X :type Float%20%28double-precision%29) (Y :type Float%20%28double-precision%29) (Z :type Float%20%28double-precision%29))
  (Transformation|SetActorRelativeLocation (Math|Vector|MakeVector X Y (+ Z (Variables|Default|GetJumpSpeed)))))

(fn MovetoPoind
  (bind _returnvalue (Transformation|GetActorLocation))
  (bind _jumppoint (Variables|Default|GetJumpPoint))
  (bind _jumppoint_2 (Variables|Default|GetJumpPoint))
  (Transformation|SetActorRelativeLocation (Math|Vector|MakeVector (.x _jumppoint) (.y _jumppoint) (.z (Transformation|GetActorLocation))))
  (if (Class|KismetMathLibrary|EqualExactlyVectorVector (Math|Vector|MakeVector (.x _jumppoint_2) (.y _jumppoint_2) 0.0) (Math|Vector|MakeVector (.x _returnvalue) (.y _returnvalue) 0.0))
    (Variables|Default|SetIsFalling true)
    (Variables|Default|SetCanJump false)))

(fn Land
  (params (X :type Float%20%28double-precision%29) (Y :type Float%20%28double-precision%29) (Z :type Float%20%28double-precision%29))
  (Transformation|SetActorRelativeLocation (Math|Vector|MakeVector X Y (- Z (Variables|Default|GetJumpSpeed)))))

(fn ResetAnimVars
  (Variables|Animation|SetInAir false)
  (Variables|Animation|SetHasLanded false)
  (Variables|Animation|SetJumpStarted false))