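; BP_TrappedPiranha is a trapped piranha actor that rises from its starting height after an animation finishes.
; BeginPlay stores the original Z, and Tick waits for the IsAnimationFinished flag, which nothing in these graphs sets.
; Once the flag is true, Tick raises Z one increment per frame until just past 200 units above the start, so speed depends on frame rate.
; It feeds world location into SetActorRelativeLocation.
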(event EventBeginPlay
  (Variables|Default|SetOriginalZLocation (.z (Transformation|GetActorLocation self))))

(event EventTick
  (params (DeltaSeconds :type Float%20%28single-precision%29))
  (bind _self self)
  (bind _returnvalue (Transformation|GetActorLocation _self))
  (if (== (Variables|Default|GetIsAnimationFinished) true)
    (if (<= (.z _returnvalue) (+ (Variables|Default|GetOriginalZLocation) 2e+02))
      (bind _result (Math|Float|IncrementFloat (.z _returnvalue))
        (:%20%20
          (Transformation|SetActorRelativeLocation (Math|Vector|MakeVector (.x _returnvalue) (.y _returnvalue) _result)))))))

(fn ConstructionScript)